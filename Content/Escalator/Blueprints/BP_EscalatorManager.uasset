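; Manager actor, one per scene, that unifies the Tick of all BP_Escalator actors to improve performance.
; Gathers the escalators in the construction script and on BeginPlay, then calls UpdateEscalators every tick.
; When AnimateInSequencer is on, Tick also copies that flag and AnimationPhase to each escalator and runs AnimateEscalator.
; The construction script does the same push regardless of the flag, updating escalators at edit time.
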(event EventBeginPlay
  ;[1 1 1] Store Escalators for Later use
  (bind _outactors (Actor|GetAllActorsOfClass "/Game/Escalator/Blueprints/BP_Escalator.BP_Escalator_C"))
  (Variables|Default|SetEscalators _outactors))

(event EventTick
  (params (DeltaSeconds :type Float%20%28single-precision%29))
  ;[1 1 1] The manager unifies the Tick event to improve performance. Add one to each scene you want to unify it.
  (Default|CallUpdateEscalators)
  ;[1 1 1] If Animated in Sequencer
  (if (Variables|Default|GetAnimate%20in%20Sequencer)
    (for _array_element (Variables|Default|GetEscalators)
      (Variables|/Game/Escalator/Blueprints/BP_Escalator.BP_Escalator_C|SetAnimate%20in%20Sequencer _array_element (Variables|Default|GetAnimate%20in%20Sequencer))
      (Variables|/Game/Escalator/Blueprints/BP_Escalator.BP_Escalator_C|SetAnimation%20Phase _array_element (Variables|Default|GetAnimation%20Phase))
      (Default|AnimateEscalator _array_element))))

(fn ConstructionScript
  (bind _outactors (Actor|GetAllActorsOfClass "/Game/Escalator/Blueprints/BP_Escalator.BP_Escalator_C"))
  (bind _output_get (Variables|Default|SetEscalators _outactors))
  (for _array_element _output_get
    (Variables|/Game/Escalator/Blueprints/BP_Escalator.BP_Escalator_C|SetAnimate%20in%20Sequencer _array_element (Variables|Default|GetAnimate%20in%20Sequencer))
    (Variables|/Game/Escalator/Blueprints/BP_Escalator.BP_Escalator_C|SetAnimation%20Phase _array_element (Variables|Default|GetAnimation%20Phase))
    (Default|AnimateEscalator _array_element)))