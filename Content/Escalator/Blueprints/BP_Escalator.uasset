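; Modular escalator or flat travelator actor with moving steps and scrolling handrails, optionally running only while the player is nearby.
; Construction script assembles end and repeated middle modules, spawns steps and fits the capsule trigger between both ends.
; AnimateEscalator loops steps by modulo of AnimationPhase, deriving escalator height from X; the phase can come from Sequencer.
; A BP_EscalatorManager, when present, drives animation instead of Tick.
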(event OnComponentBeginOverlap(Enabler)
  (params (OverlappedComponent :type Primitive%20Component%20Object%20Reference) (OtherActor :type Actor%20Object%20Reference) (OtherComp :type Primitive%20Component%20Object%20Reference) (OtherBodyIndex :type Integer) (bFromSweep :type Boolean) (SweepResult :type Hit%20Result%20Structure%20%28by%20ref%29))
  (if (== OtherActor (Game|Player|GetPlayerPawn 0))
    (Variables|Default|SetisEnabled true)))

(event OnComponentEndOverlap(Enabler)
  (params (OverlappedComponent :type Primitive%20Component%20Object%20Reference) (OtherActor :type Actor%20Object%20Reference) (OtherComp :type Primitive%20Component%20Object%20Reference) (OtherBodyIndex :type Integer))
  (if (== (Game|Player|GetPlayerPawn 0) OtherActor)
    (Variables|Default|SetisEnabled false)))

(event Custom|Animate
  (CallFunction|AnimateEscalator))

(event EventBeginPlay
  (if (Variables|Escalator|Parameters|GetUse%20Proximity%20to%20Activate)
    (Variables|Default|SetisEnabled (Collision|IsOverlappingActor (Variables|Default|GetEnabler) (Game|Player|GetPlayerPawn 0) :!class /Script/Engine.PrimitiveComponent)))
  (bind _outactors (Actor|GetAllActorsOfClass "/Game/Escalator/Blueprints/BP_EscalatorManager.BP_EscalatorManager_C"))
  (if (Utilities|Array|IsValidIndex _outactors)
    (EventDispatchers|BindEventtoUpdateEscalators (Utilities|Array|Get(acopy) _outactors) (delegate Custom|Animate))
    (Variables|Default|SetHas%20Manager true)
    (Actor|Tick|SetActorTickEnabled false)
    (else
      (Variables|Default|SetHas%20Manager false))))

(event EventTick
  (params (DeltaSeconds :type Float%20%28single-precision%29))
  ;[1 1 1] Tick
  (if (not (Variables|Default|GetHas%20Manager))
    (CallFunction|AnimateEscalator)))

(fn ConstructionScript
  (bind _beginning (Variables|Default|GetBeginning))
  (bind _beginning_2 (Variables|Default|GetBeginning))
  (bind _ending (Variables|Default|GetEnding))
  (bind _beginning_3 (Variables|Default|GetBeginning))
  (bind _ending_2 (Variables|Default|GetEnding))
  (bind _ending_3 (Variables|Default|GetEnding))
  (bind _enabler (Variables|Default|GetEnabler))
  (bind _extra_steps_travelator (Variables|Default|GetExtra%20Steps%20Travelator))
  (bind _extra_steps_escalator (Variables|Default|GetExtra%20Steps%20Escalator))
  (bind _extension (Variables|Escalator|Parameters|GetExtension))
  (bind _relativelocation (Variables|/Script/Engine.SceneComponent|GetRelativeLocation _beginning_2))
  (bind _relativelocation_2 (Variables|/Script/Engine.SceneComponent|GetRelativeLocation _ending))
  (bind _relativelocation_3 (Variables|/Script/Engine.SceneComponent|GetRelativeLocation _beginning_3))
  (bind _relativelocation_4 (Variables|/Script/Engine.SceneComponent|GetRelativeLocation _ending_2))
  (bind _relativelocation_5 (Variables|/Script/Engine.SceneComponent|GetRelativeLocation _ending_3))
  (bind _relativelocation_6 (Variables|/Script/Engine.SceneComponent|GetRelativeLocation _beginning))
  (bind _returnvalue (- _relativelocation _relativelocation_2))
  (bind _returnvalue_2 (- _relativelocation_3 _relativelocation_4))
  (bind _returnvalue_3 (Math|Vector|VectorLength _returnvalue))
  (bind _returnvalue_4 (Math|Vector|VectorLength _returnvalue_2))
  (bind _returnvalue_5 (/ _returnvalue_3 32.5))
  (bind _returnvalue_6 (/ _returnvalue_4 32.5))
  (bind _returnvalue_7 (Math|Float|Ceil _returnvalue_6))
  (bind _returnvalue_8 (Math|Float|Ceil _returnvalue_5))
  (bind _returnvalue_9 (+ _returnvalue_7 _extra_steps_escalator))
  (bind _returnvalue_10 (+ _returnvalue_8 _extra_steps_travelator))
  (Utilities|FlowControl|Sequence
    (:then_0
      ;[1 1 1] Static Mesh Modules
      (for (_array_element _array_index) (Utilities|Array|MakeArray (Variables|Default|GetBeginning) (Variables|Default|GetBeginningFloor) (Variables|Default|GetElevationStart) (Variables|Default|GetRubberSegment01) (Variables|Default|GetEnding) (Variables|Default|GetEndingFloor) (Variables|Default|GetElevationEnd) (Variables|Default|GetRubberSegment02))
        (Utilities|IsValid _array_element
          (:Is%20Valid
            (Components|StaticMesh|SetStaticMesh _array_element (Utilities|Array|Get(acopy) (Utilities|Array|MakeArray (Variables|Escalator|Modules|GetBeginning%20Module) (Variables|Escalator|Modules|GetBeginning%20Floor) (Variables|Escalator|Modules|GetElevation%20Start) (Variables|Escalator|Modules|GetHandrail%20Segment%2001) (Variables|Escalator|Modules|GetEnding%20Module) (Variables|Escalator|Modules|GetEnding%20Floor) (Variables|Escalator|Modules|GetElevation%20End) (Variables|Escalator|Modules|GetHandrail%20Segment%2002)) _array_index)))))
      ;[1 1 1] Material Management
      (bind _returnvalue_11 (Rendering|Material|CreateDynamicMaterialInstance "/Game/Escalator/Materials/MI_Escalator_Rubber.MI_Escalator_Rubber" "Handrail" "None" :!class /Script/Engine.KismetMaterialLibrary))
      (Variables|Default|SetHandrail%20Material _returnvalue_11)
      (for _array_element_2 (Utilities|Array|MakeArray (Variables|Default|GetElevationStart) (Variables|Default|GetEnding) (Variables|Default|GetElevationEnd) (Variables|Default|GetBeginning))
        (Rendering|Material|SetMaterial _array_element_2 (Rendering|Material|GetMaterialIndex _array_element_2 "Rubber") (Variables|Default|GetHandrail%20Material)))
      ;[1 1 1] Clear Array
      (Utilities|Array|Clear (Variables|Default|GetSteps))
      ;[1 1 1] Switch Inclination Modules
      (if (Variables|Escalator|Parameters|GetEscalator)
        (Components|DestroyComponent (Variables|Default|GetRubberSegment01))
        (else
          (Components|DestroyComponent (Variables|Default|GetElevationEnd))))
      ;[1 1 1] Array Middle Segments
      (for _index (range 0 (- (Variables|Escalator|Parameters|GetExtension) 1))
        (bind _returnvalue_12 (AddComponent|AddStaticMeshComponent false (Math|Transform|MakeTransform (select (Variables|Escalator|Parameters|GetEscalator) (+ (Variables|/Script/Engine.SceneComponent|GetRelativeLocation (Variables|Default|GetElevationStart)) (* (Variables|Parameters|Escalator|GetEscalator%20Module%20Offset) _index)) (+ (Variables|Parameters|Travelator|GetTravelator%20Module%20Global%20Offset) (* (Variables|Parameters|Travelator|GetTravelator%20Module%20Offset) _index))) "0, 0, 0" "1.000000,1.000000,1.000000")))
        (Components|StaticMesh|SetStaticMesh _returnvalue_12 (select (Variables|Escalator|Parameters|GetEscalator) (Variables|Escalator|Modules|GetInclination%20Segment) (Variables|Escalator|Modules|GetHorizontal%20Segment)))
        (Rendering|Material|SetMaterial _returnvalue_12 (Rendering|Material|GetMaterialIndex _returnvalue_12 "Rubber") (Variables|Default|GetHandrail%20Material))
        (bind _returnvalue_13 (AddComponent|AddStaticMeshComponent false (Math|Transform|MakeTransform (select (Variables|Escalator|Parameters|GetEscalator) (+ (Variables|/Script/Engine.SceneComponent|GetRelativeLocation (Variables|Default|GetElevationStart)) (* (Variables|Parameters|Escalator|GetEscalator%20Module%20Offset) _index)) (+ (Variables|Parameters|Travelator|GetTravelator%20Module%20Global%20Offset) (* (Variables|Parameters|Travelator|GetTravelator%20Module%20Offset) _index))) "0, 0, 0" "1.000000,1.000000,1.000000")))
        (Components|StaticMesh|SetStaticMesh _returnvalue_13 (select (Variables|Escalator|Parameters|GetEscalator) (Variables|Escalator|Modules|GetInclination%20Segment%20-%20Glass) (Variables|Escalator|Modules|GetHorizontal%20Segment%20-%20Glass))))
      ;[1 1 1] Offset Beginning and End
      (Transformation|SetRelativeLocation (Variables|Default|GetEnding) (select (Variables|Escalator|Parameters|GetEscalator) (+ (* (Variables|Parameters|Escalator|GetEscalator%20Module%20Offset) _extension) "-259.967834,0.000000,53.380001") (+ (* (Variables|Parameters|Travelator|GetTravelator%20Module%20Offset) _extension) "-90.500000,0.000000,0.000000")) false false)
      (Utilities|FlowControl|Sequence
        (:then_0
          (Utilities|Array|Clear (Variables|Default|GetDefault%20Location))
          (if (Variables|Escalator|Parameters|GetEscalator)
            ;[1 1 1] Add Steps to Escalators
            (Variables|Default|SetAmount%20of%20Steps%20Until%20End (- _returnvalue_9 1))
            ;;[1 1 1] Offset By Step
            (for _index_2 (range 0 _returnvalue_9)
              (bind _output_get (LocalVariables|SetCurrent%20Index _index_2))
              (if (< (- (.X (Math|Vector|BreakVector (Variables|/Script/Engine.SceneComponent|GetRelativeLocation (Variables|Default|GetEnding)))) (Math|Float|Absolute(Float) (* (Variables|Default|GetExtra%20Steps%20Escalator) (Variables|Parameters|GetStep%20Offset%20%28X%29)))) (.X (Math|Vector|BreakVector (CallFunction|GetStepLocationonEscalator _output_get))))
                ;;[1 1 1] Add Static Mesh and store inside array "Steps"
                (bind _returnvalue_14 (AddComponent|AddStaticMeshComponent false (Math|Transform|MakeTransform (CallFunction|GetStepLocationonEscalator _output_get) "0, 0, 0" "1.000000,1.000000,1.000000")))
                (Components|StaticMesh|SetStaticMesh _returnvalue_14 (Variables|Escalator|Modules|GetStep%20Module))
                (Utilities|Array|Add (Variables|Default|GetSteps) _returnvalue_14)
                (Utilities|Array|Add (Variables|Default|GetDefault%20Location) (Variables|/Script/Engine.SceneComponent|GetRelativeLocation _returnvalue_14))))
            (Variables|Default|SetLast%20Step%20Location (CallFunction|GetStepLocationonEscalator _returnvalue_9))
            (else
              ;[1 1 1] Add Steps To Non Escalators
              (for _index_3 (range 0 _returnvalue_10)
                ;;[1 1 1] Add Static Mesh and store inside array "Steps"
                (bind _returnvalue_15 (AddComponent|AddStaticMeshComponent false (Math|Transform|MakeTransform (CallFunction|GetStepLocationonTravelator _index_3) "0, 0, 0" "1.000000,1.000000,1.000000")))
                (Components|StaticMesh|SetStaticMesh _returnvalue_15 (Variables|Escalator|Modules|GetStep%20Module))
                (Utilities|Array|Add (Variables|Default|GetSteps) _returnvalue_15)
                (Utilities|Array|Add (Variables|Default|GetDefault%20Location) (Variables|/Script/Engine.SceneComponent|GetRelativeLocation _returnvalue_15)))
              ;;[1 1 1] Store Last Step Location
              (Variables|Default|SetLast%20Step%20Location (CallFunction|GetStepLocationonEscalator _returnvalue_10)))))
        (:then_1
          ;[1 1 1] Create Activation Trigger
          (if (Variables|Escalator|Parameters|GetUse%20Proximity%20to%20Activate)
            (Components|Capsule|SetCapsuleHalfHeight _enabler (Math|Vector|Distance(Vector) _relativelocation_6 _relativelocation_5) true)
            (Components|Capsule|SetCapsuleRadius _enabler (Variables|Escalator|Parameters|GetProximity%20Radius) true)
            (Transformation|SetRelativeLocationAndRotation (Variables|Default|GetEnabler) (+ _relativelocation_5 (/ (- _relativelocation_6 _relativelocation_5) 2.0)) (Math|Rotator|CombineRotators (Math|Rotator|FindLookatRotation _relativelocation_6 _relativelocation_5) "90.000000, 0, 0") false false)
            (else
              (Variables|Default|SetisEnabled true)
              (Components|DestroyComponent (Variables|Default|GetEnabler)))))))
    (:then_1
      (CallFunction|AnimateEscalator))))

(fn AnimateEscalator
  (bind _default_location (Variables|Default|GetDefault%20Location))
  (bind _step_offset__x_ (Variables|Parameters|GetStep%20Offset%20%28X%29))
  (bind _steps (Variables|Default|GetSteps))
  (bind _default_location_2 (Variables|Default|GetDefault%20Location))
  (bind _default_location_3 (Variables|Default|GetDefault%20Location))
  (bind _returnvalue (Utilities|Array|LastIndex _default_location))
  (bind _returnvalue_2 (Utilities|Array|Length _steps))
  (bind _returnvalue_3 (Math|Float|Absolute(Float) _step_offset__x_))
  (bind _output (Utilities|Array|Get(acopy) _default_location))
  (bind _x (Math|Vector|BreakVector _output))
  (bind _returnvalue_4 (* _returnvalue_2 _returnvalue_3))
  (bind _output_2 (Utilities|Array|Get(acopy) _default_location _returnvalue))
  (bind _x_2 (Math|Vector|BreakVector _output_2))
  (bind _returnvalue_5 (- _x_2 _x))
  (bind _returnvalue_6 (Math|Float|Absolute(Float) _returnvalue_5))
  (if (Variables|Default|GetisEnabled)
    (if (Variables|Escalator|GetAnimate%20in%20Sequencer)
      _
      (else
        (Variables|Escalator|SetAnimation%20Phase (+ (Variables|Escalator|GetAnimation%20Phase) (Utilities|Time|GetWorldDeltaSeconds)))))
    (Rendering|Material|SetScalarParameterValue (Variables|Default|GetHandrail%20Material) "V Speed" (* (Variables|Escalator|Parameters|GetSpeed) 2.0 (Math|Float|Lerp 1.0 -1.0 (Math|Conversions|ToFloat(Boolean) (Variables|Escalator|GetSwitch%20Direction)))) :!class /Script/Engine.MaterialInstanceDynamic)
    (if (Variables|Escalator|Parameters|GetEscalator)
      ;[1 1 1] Move Escalator
      (for (_array_element _array_index) (Variables|Default|GetSteps)
        (Transformation|SetRelativeLocation _array_element (Math|Vector|MakeVector (.X (Math|Vector|BreakVector (CallFunction|GetEscalatorLocationfromX (select (Variables|Escalator|GetSwitch%20Direction) (- (.X (Math|Vector|BreakVector (Utilities|Array|Get(acopy) _default_location_3))) (Math|Float|%(Float) (+ (.X (Math|Vector|BreakVector (Utilities|Array|Get(acopy) (Variables|Default|GetDefault%20Location) _array_index))) _returnvalue_6 (* (Variables|Escalator|Parameters|GetSpeed) (Variables|Escalator|GetAnimation%20Phase) 1e+02)) _returnvalue_6)) (+ (.X (Math|Vector|BreakVector (Utilities|Array|Get(acopy) _default_location_3 (Utilities|Array|LastIndex _default_location_3)))) (Math|Float|%(Float) (+ (.X (Math|Vector|BreakVector (Utilities|Array|Get(acopy) (Variables|Default|GetDefault%20Location) _array_index))) _returnvalue_6 (* (Variables|Escalator|Parameters|GetSpeed) (Variables|Escalator|GetAnimation%20Phase) 1e+02)) _returnvalue_6)))))) (.Y (Math|Vector|BreakVector (Utilities|Array|Get(acopy) (Variables|Default|GetDefault%20Location) _array_index))) (.Z (Math|Vector|BreakVector (CallFunction|GetEscalatorLocationfromX (select (Variables|Escalator|GetSwitch%20Direction) (- (.X (Math|Vector|BreakVector (Utilities|Array|Get(acopy) _default_location_3))) (Math|Float|%(Float) (+ (.X (Math|Vector|BreakVector (Utilities|Array|Get(acopy) (Variables|Default|GetDefault%20Location) _array_index))) _returnvalue_6 (* (Variables|Escalator|Parameters|GetSpeed) (Variables|Escalator|GetAnimation%20Phase) 1e+02)) _returnvalue_6)) (+ (.X (Math|Vector|BreakVector (Utilities|Array|Get(acopy) _default_location_3 (Utilities|Array|LastIndex _default_location_3)))) (Math|Float|%(Float) (+ (.X (Math|Vector|BreakVector (Utilities|Array|Get(acopy) (Variables|Default|GetDefault%20Location) _array_index))) _returnvalue_6 (* (Variables|Escalator|Parameters|GetSpeed) (Variables|Escalator|GetAnimation%20Phase) 1e+02)) _returnvalue_6))))))) false false))
      (else
        ;[1 1 1] Move Travelator
        (for (_array_element_2 _array_index_2) (Variables|Default|GetSteps)
          (Transformation|SetRelativeLocation _array_element_2 (Math|Vector|MakeVector (select (Variables|Escalator|GetSwitch%20Direction) (- (.X (Math|Vector|BreakVector (Utilities|Array|Get(acopy) _default_location_2))) (Math|Float|%(Float) (+ (.X (Math|Vector|BreakVector (Utilities|Array|Get(acopy) (Variables|Default|GetDefault%20Location) _array_index_2))) _returnvalue_4 (* (Variables|Escalator|Parameters|GetSpeed) (Variables|Escalator|GetAnimation%20Phase) 1e+02)) _returnvalue_4)) (+ (.X (Math|Vector|BreakVector (Utilities|Array|Get(acopy) _default_location_2 (Utilities|Array|LastIndex _default_location_2)))) (Math|Float|%(Float) (+ (.X (Math|Vector|BreakVector (Utilities|Array|Get(acopy) (Variables|Default|GetDefault%20Location) _array_index_2))) _returnvalue_4 (* (Variables|Escalator|Parameters|GetSpeed) (Variables|Escalator|GetAnimation%20Phase) 1e+02)) _returnvalue_4))) (.Y (Math|Vector|BreakVector (Utilities|Array|Get(acopy) (Variables|Default|GetDefault%20Location) _array_index_2))) (.Z (Math|Vector|BreakVector (Utilities|Array|Get(acopy) (Variables|Default|GetDefault%20Location) _array_index_2)))) false false))))))

(fn GetStepLocationonEscalator
  (params (Index :type Integer))
  (return (CallFunction|GetEscalatorLocationfromX (* Index (Variables|Parameters|GetStep%20Offset%20%28X%29)))))

(fn GetStepLocationonTravelator
  (params (Index :type Integer))
  (return (+ (Variables|Parameters|Travelator|GetTravelator%20Steps%20Global%20Offset) (Math|Vector|MakeVector (* Index (Variables|Parameters|GetStep%20Offset%20%28X%29)) 0.0 0.0))))

(fn GetAnimationOffset
  (params (Old%20Position :type Vector))
  (bind _speed (Variables|Escalator|Parameters|GetSpeed))
  (return (+ Old%20Position (Math|Vector|MakeVector (Math|Float|Lerp _speed (- 0.0 _speed) (Math|Conversions|ToFloat(Boolean) (Variables|Escalator|GetSwitch%20Direction))) 0.0 0.0))))

(fn GetEscalatorLocationfromX
  (params (X :type Float%20%28double-precision%29))
  (return (+ (Variables|Default|GetFirst%20Step%20Location) (Math|Vector|MakeVector X 0.0 (Math|Float|Clamp(Float) (+ (* X (Math|Trig|Sin(Degrees) (Variables|Parameters|GetEscalator%20Inclination)) -1.0) (Variables|Parameters|GetSteps%20Elevation%20Offset)) 0.0 (.Z (Math|Vector|BreakVector (Variables|/Script/Engine.SceneComponent|GetRelativeLocation (Variables|Default|GetEnding)))))))))